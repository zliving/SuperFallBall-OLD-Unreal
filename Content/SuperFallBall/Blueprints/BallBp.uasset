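; BallBp is the player-steered ball for SuperFallBall, moved sideways with the Left and Right keys.
; BeginPlay enables player input, and key press and release events set held-state flags.
; Tick reads those flags to teleport-free nudge the ball along X by a fixed step per frame without sweep and roll it around pitch.
; Movement is frame-rate dependent, and Left takes priority when both keys are held.
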(event EventBeginPlay
  ;[1 1 1] Enable input and set current location
  (Input|EnableInput (Game|GetPlayerController 0)))

(event EventActorBeginOverlap
  (params (OtherActor :type Actor%20Object%20Reference))
  ;[1 1 1] Enable input and set current location
)

(event EventTick
  (params (DeltaSeconds :type Float%20%28single-precision%29))
  ;[1 1 1] Update location and rotate if left or right is pressed
  (Variables|Default|SetballLocation (Transformation|GetActorLocation))
  (if (Variables|Default|GetleftPressed)
    (Transformation|SetActorLocation (+ (Variables|Default|GetballLocation) "-5.000000, 0, 0") false false)
    (Transformation|AddActorLocalRotation (Math|Rotator|MakeRotator 0.0 5.0 0.0) false false)
    (elif (Variables|Default|GetrightPressed)
      (Transformation|SetActorLocation (+ (Variables|Default|GetballLocation) "5.000000, 0, 0") false false)
      (Transformation|AddActorLocalRotation (Math|Rotator|MakeRotator 0.0 -5.0 0.0) false false))))

(event Input|KeyboardEvents|Left
  (params (Key :type Key%20Structure :default "AnyKey"))
  ;[1 1 1] Set isPressed to true if a key is pressed
  (:Pressed
    (Variables|Default|SetleftPressed true))
  (:Released
    (Variables|Default|SetleftPressed false)))

(event Input|KeyboardEvents|Right
  (params (Key :type Key%20Structure :default "AnyKey"))
  ;[1 1 1] Set isPressed to true if a key is pressed
  (:Pressed
    (Variables|Default|SetrightPressed true))
  (:Released
    (Variables|Default|SetrightPressed false)))

(fn ConstructionScript)